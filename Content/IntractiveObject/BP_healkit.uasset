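; BP_healkit is an interactive health pickup that heals the player's third-person character.
; On Interact, it adds a fixed amount to Health unless Health exactly equals the full value, with no clamp on the result.
; It then pushes the new value to the HealthBar widget held by BP_ThirdPersonGameMode and destroys itself.
; At full health, the interaction does nothing and the kit remains.
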(event `self.interact`
  (bind _asbp_third_person_character (cast `/Game/ThirdPerson/Blueprints/BP_ThirdPersonCharacter` (`GameplayStatics.GetPlayerCharacter` 0)))
  (if (not (== (`/Game/ThirdPerson/Blueprints/BP_ThirdPersonCharacter.health` _asbp_third_person_character) 100.0))
    (bind _output_get (set `/Game/ThirdPerson/Blueprints/BP_ThirdPersonCharacter.health` (+ 15.0 (`/Game/ThirdPerson/Blueprints/BP_ThirdPersonCharacter.health` _asbp_third_person_character)) _asbp_third_person_character))
    (bind _asbp_third_person_game_mode (cast `/Game/ThirdPerson/Blueprints/BP_ThirdPersonGameMode` (`GameplayStatics.GetGameMode`)))
    (`/Game/IntractiveObject/UI_health.update heath` (`/Game/ThirdPerson/Blueprints/BP_ThirdPersonGameMode.health bar` _asbp_third_person_game_mode) _output_get)
    (`self.K2_DestroyActor`)))

(fn `UserConstructionScript`
  (`parent.UserConstructionScript`))